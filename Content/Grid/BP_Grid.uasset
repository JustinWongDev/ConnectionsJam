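; Grid actor that builds the puzzle board of socket tiles framed by bulb tiles, then lights coloured bulb pairs on a timer.
; Init reads board size from the game mode's settings and spawns tiles on the Y-Z plane, skipping corners.
; A looping timer picks two random bulb tiles, which may coincide, assigns an unused colour and records the pair.
; Separate, locally uncalled events pair fixed-index bulbs with same-row or same-column partners.
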(event Custom|SpawnBoard
  (bind _gm (Variables|Ref|GetGM))
  (bind _gamesettings (Variables|/Game/Game/BP_GameMode.BP_GameMode_C|GetGameSettings _gm))
  (bind (_socketrows _socketcolumns) (Utilities|Struct|BreakS_GameSettings _gamesettings))
  (bind _returnvalue (+ _socketrows 1))
  (bind _returnvalue_2 (+ _socketcolumns 1))
  (for _index (range 0 _returnvalue)
    (for _index_2 (range 0 _returnvalue_2)
      (if (Math|Boolean|ORBoolean (== _index 0) (== _index_2 0) (== _index _returnvalue) (== _index_2 _returnvalue_2))
        (CallFunction|BulbTileCheck _index _index_2)
        (else
          (CallFunction|SpawnSocketTile _index _index_2))))))

(event Custom|SpawnOppositeCOlumn
  (bind _bulbtilearray (Variables|Data|GetBulbTileArray))
  (bind _output (Utilities|Array|Get(acopy) _bulbtilearray 4))
  (bind _output_get (Variables|Temp|SetTempColour (Math|Vector|MakeVector (Math|Random|RandomFloatinRange 0.0 1.0) (Math|Random|RandomFloatinRange 0.0 1.0) (Math|Random|RandomFloatinRange 0.0 1.0))))
  (bind _tile (CallFunction|GetSameColumnTile (Variables|/Game/Grid/BP_Tile.BP_Tile_C|GetColumn _output) _output))
  (Utilities|Array|AddUnique (Variables|Data|GetBulbPairs) (Utilities|Struct|MakeS_Pairs _output _tile (Math|Conversions|ToLinearColor(Vector) _output_get)))
  (Default|SetBulb _output true (Variables|Temp|GetTempColour) (Utilities|Struct|MakeS_Pairs _output _tile (Math|Conversions|ToLinearColor(Vector) _output_get)))
  (Default|SetBulb _tile true (Variables|Temp|GetTempColour) (Utilities|Struct|MakeS_Pairs _output _tile (Math|Conversions|ToLinearColor(Vector) _output_get))))

(event Custom|SpawnOppositeRow
  (bind _bulbtilearray (Variables|Data|GetBulbTileArray))
  (bind _returnvalue (Utilities|Array|Length _bulbtilearray))
  (bind _returnvalue_2 (- _returnvalue 1))
  (bind _returnvalue_3 (- _returnvalue_2 5))
  (bind _output (Utilities|Array|Get(acopy) _bulbtilearray _returnvalue_3))
  (bind _output_get (Variables|Temp|SetTempColour (Math|Vector|MakeVector (Math|Random|RandomFloatinRange 0.0 1.0) (Math|Random|RandomFloatinRange 0.0 1.0) (Math|Random|RandomFloatinRange 0.0 1.0))))
  (bind _tile (CallFunction|GetSameRowTile (Variables|/Game/Grid/BP_Tile.BP_Tile_C|GetRow _output) _output))
  (Utilities|Array|AddUnique (Variables|Data|GetBulbPairs) (Utilities|Struct|MakeS_Pairs _output _tile (Math|Conversions|ToLinearColor(Vector) _output_get)))
  (Default|SetBulb _output true (Variables|Temp|GetTempColour) (Utilities|Struct|MakeS_Pairs _output _tile (Math|Conversions|ToLinearColor(Vector) _output_get)))
  (Default|SetBulb _tile true (Variables|Temp|GetTempColour) (Utilities|Struct|MakeS_Pairs _output _tile (Math|Conversions|ToLinearColor(Vector) _output_get))))

(event Custom|SpawnBulbPair
  (CallFunction|SpawnRandomBulbPair))

(event Custom|SpawnRandomBulbPair
  (bind _bulbtilearray (Variables|Data|GetBulbTileArray))
  (Variables|Temp|SetTempColour (Math|Vector|MakeVector (Math|Random|RandomFloatinRange 0.0 1.0) (Math|Random|RandomFloatinRange 0.0 1.0) (Math|Random|RandomFloatinRange 0.0 1.0)))
  (Variables|Temp|SetTempPair (Utilities|Struct|MakeS_Pairs (Utilities|Array|Get(acopy) _bulbtilearray (Math|Random|RandomIntegerinRange 0 (- (Utilities|Array|Length _bulbtilearray) 1))) (Utilities|Array|Get(acopy) _bulbtilearray (Math|Random|RandomIntegerinRange 0 (- (Utilities|Array|Length _bulbtilearray) 1))) (Utilities|Struct|BreakS_BulbColours (CallFunction|GetUnusedColour))))
  (Default|SetBulb (.FirstTile (Utilities|Struct|BreakS_Pairs (Variables|Temp|GetTempPair))) true (Math|Conversions|ToVector(LinearColor) (.Colour (Utilities|Struct|BreakS_Pairs (Variables|Temp|GetTempPair)))) (Variables|Temp|GetTempPair))
  (Default|SetBulb (.LastTile (Utilities|Struct|BreakS_Pairs (Variables|Temp|GetTempPair))) true (Math|Conversions|ToVector(LinearColor) (.Colour (Utilities|Struct|BreakS_Pairs (Variables|Temp|GetTempPair)))) (Variables|Temp|GetTempPair))
  (Utilities|Array|AddUnique (Variables|Data|GetBulbPairs) (Variables|Temp|GetTempPair)))

(event Custom|BulbTileCheck
  (params (Row :type Integer) (Column :type Integer))
  (bind _gm (Variables|Ref|GetGM))
  (bind _gamesettings (Variables|/Game/Game/BP_GameMode.BP_GameMode_C|GetGameSettings _gm))
  (bind (_socketrows _socketcolumns) (Utilities|Struct|BreakS_GameSettings _gamesettings))
  (bind _returnvalue (+ _socketrows 1))
  (bind _returnvalue_2 (+ _socketcolumns 1))
  (if (not (Math|Boolean|ORBoolean (and (== Row 0) (== Column 0)) (and (== Row 0) (== Column _returnvalue_2)) (and (== Row _returnvalue) (== Column 0)) (and (== Row _returnvalue) (== Column _returnvalue_2))))
    (CallFunction|SpawnBulbTile Column Row)))

(event Custom|SpawnSocketTile
  (params (Row :type Integer) (Column :type Integer))
  (bind _returnvalue (Transformation|GetActorLocation))
  (bind (_x _y _z) (Math|Vector|BreakVector _returnvalue))
  (bind _returnvalue_2 (Game|SpawnActorfromClass "/Game/Grid/BP_SocketTile.BP_SocketTile_C" (Math|Transform|MakeTransform (Math|Vector|MakeVector _x (+ _y (* (Math|Conversions|ToFloat(Integer) Column) (Variables|Default|GetDistanceBetweenTiles))) (- _z (* (Math|Conversions|ToFloat(Integer) Row) (Variables|Default|GetDistanceBetweenTiles))))) "Undefined" 0 0))
  (Default|Init _returnvalue_2 Row Column)
  (Utilities|Array|AddUnique (Variables|Data|GetAllTileArray) _returnvalue_2))

(event Custom|SpawnBulbTile
  (params (Row :type Integer) (Column :type Integer))
  (bind _returnvalue (Transformation|GetActorLocation))
  (bind (_x _y _z) (Math|Vector|BreakVector _returnvalue))
  (bind _returnvalue_2 (Game|SpawnActorfromClass "/Game/Grid/BP_BulbTile.BP_BulbTile_C" (Math|Transform|MakeTransform (Math|Vector|MakeVector _x (+ _y (* (Math|Conversions|ToFloat(Integer) Row) (Variables|Default|GetDistanceBetweenTiles))) (- _z (* (Math|Conversions|ToFloat(Integer) Column) (Variables|Default|GetDistanceBetweenTiles))))) "Undefined" 0 0))
  (Default|Init _returnvalue_2 Column Row)
  (Utilities|Array|AddUnique (Variables|Data|GetBulbTileArray) _returnvalue_2)
  (Utilities|Array|AddUnique (Variables|Data|GetAllTileArray) _returnvalue_2))

(event Custom|Init
  (bind _asbp_game_mode (Utilities|Casting|CastToBP_GameMode (Game|GetGameMode)))
  (Variables|Ref|SetGM _asbp_game_mode)
  (CallFunction|SpawnBoard)
  (Utilities|Time|SetTimerbyEvent (delegate Custom|SpawnBulbPair) (.TimeBetweenPairs (Utilities|Struct|BreakS_GameSettings (CallFunction|GetGameSettings))) true))

(fn ConstructionScript)

(fn GetSameColumnTile
  (params (Column :type Integer) (BulbTile :type BP%20Bulb%20Tile%20Object%20Reference))
  (for _array_element (Variables|Data|GetBulbTileArray)
    (if (and (== (Variables|/Game/Grid/BP_Tile.BP_Tile_C|GetColumn _array_element) Column) (!= BulbTile _array_element))
      (return _array_element)))
  (return 0))

(fn GetSameRowTile
  (params (Row :type Integer) (BulbTile :type BP%20Bulb%20Tile%20Object%20Reference))
  (for _array_element (Variables|Data|GetBulbTileArray)
    (if (and (== (Variables|/Game/Grid/BP_Tile.BP_Tile_C|GetRow _array_element) Row) (!= BulbTile _array_element))
      (return _array_element)))
  (return 0))