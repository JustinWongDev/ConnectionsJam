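; BP_SocketTile is a grid tile that can hold a plug and tracks whether it sits next to a bulb tile.
; It starts unplugged; SetPlug toggles the plug mesh's visibility and rechecks bulb adjacency from its row and column.
; When a neighboring bulb is found, it caches that tile and binds to its OnBulbGone event, with a separate function to clear the cached state.
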(event EventBeginPlay
  (CallFunction|SetPlug false))

(fn ConstructionScript
  (|CallParentFunction))

(fn SetPlug
  (params (Has%20Plug :type Boolean))
  (bind _output_get (Variables|Default|SetHasPlug Has%20Plug))
  (Rendering|SetVisibility (Variables|Default|GetPlugMesh) _output_get true)
  (CallFunction|CheckNexttoBulbState)
  (return (Variables|Default|GetHasPlug)))

(fn RemoveNexttoBulbState
  (Variables|Default|SetNextToBulb false)
  (Variables|Default|SetBulbTile 0))

(fn CheckNexttoBulbState
  (bind _row (Variables|Default|GetRow))
  (bind _column (Variables|Default|GetColumn))
  (bind (_next_to_bulb _bulbtile) (CallFunction|AdjacenttoBulb _row _column))
  (bind _output_get (Variables|Default|SetNextToBulb _next_to_bulb))
  (Variables|Default|SetBulbTile _bulbtile)
  (if _output_get
    (EventDispatchers|BindEventtoOnBulbGone (Variables|Default|GetBulbTile) (EventDispatchers|CreateEvent :!event RemoveNexttoBulbState)))
  (return))