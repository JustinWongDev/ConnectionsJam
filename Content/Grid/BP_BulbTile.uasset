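; Grid tile that can hold a coloured light bulb in what appears to be a path puzzle.
; SetBulb swaps tile and bulb meshes, stores colour and pair, starts the bulb, and notifies an adjacent plug's socket tile.
; A slowed timeline scales light intensity and radius while blending the colour toward a warning colour.
; When it finishes, the tile runs a path check, clears the bulb after a short delay and signals it is gone.
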(event Custom|Start
  (bind _pointlight (Variables|Default|GetPointLight))
  (bind _initialcolour (Variables|Setup|GetInitialColour))
  (bind _pointlight_2 (Variables|Default|GetPointLight))
  (bind (_x _y _z) (Math|Vector|BreakVector _initialcolour))
  (Variables|Setup|SetInitialIntensity (Variables|/Script/Engine.LightComponentBase|GetIntensity _pointlight_2))
  (Variables|Setup|SetInitialAttenuation (Variables|/Script/Engine.LocalLightComponent|GetAttenuationRadius _pointlight_2))
  (Components|Timeline|SetPlayRate (Variables|Default|GetBrightnessTimeline) 0.1)
  (bind (_direction _brightness _colour _warningcolour) (Timeline|BrightnessTimeline PlayFromStart)
    (:Update
      (Rendering|Components|Light|SetIntensity _pointlight (* (Variables|Setup|GetInitialIntensity) _brightness))
      (Rendering|Lighting|SetAttenuationRadius _pointlight (* (Variables|Setup|GetInitialAttenuation) _brightness))
      (Rendering|Material|SetVectorParameterValueonMaterials (Variables|Default|GetBulbMesh) "Colour" (Math|Conversions|ToVector(LinearColor) (Math|Color|Lerp(LinearColor) (Utilities|Struct|MakeLinearColor _x _y _z 1.0) (Variables|Setup|GetWarningColour) _warningcolour)))
      (Rendering|Components|Light|SetLightColor (Variables|Default|GetPointLight) (Math|Color|Lerp(LinearColor) (Utilities|Struct|MakeLinearColor _x _y _z 1.0) (Variables|Setup|GetWarningColour) _warningcolour) true))
    (:Finished
      ;[1 1 1] JW TODO
      ; Replace algorithm?
      (CallFunction|CheckforPath self)
      (Utilities|FlowControl|Delay 0.2)
      (CallFunction|SetBulb false "0, 0, 0")
      (Default|CallOnBulbGone))))

(event EventBeginPlay
  (CallFunction|SetBulb false "0, 0, 0"))

(fn ConstructionScript
  (|CallParentFunction))

(fn SetBulb
  (params (State :type Boolean) (Colour :type Vector) (BulbPair :type S%20Pairs%20Structure))
  (bind _row (Variables|Default|GetRow))
  (bind _column (Variables|Default|GetColumn))
  (bind (_next_to_plug _sockettile) (CallFunction|AdjacenttoPlug _row _column))
  (bind _output_get (Variables|Setup|SetHasBulb State))
  (Rendering|SetVisibility (Variables|Default|GetBulbMesh) _output_get true)
  (Rendering|SetVisibility (Variables|Default|GetTileMesh) (not _output_get) true)
  (Variables|Setup|SetSide (CallFunction|DetermineSide self))
  (if (Variables|Setup|GetHasBulb)
    (Variables|Setup|SetBulbPair BulbPair)
    (bind _output_get_2 (Variables|Setup|SetInitialColour Colour))
    (Rendering|Material|SetVectorParameterValueonMaterials (Variables|Default|GetBulbMesh) "Colour" _output_get_2)
    (CallFunction|Start)
    (if _next_to_plug
      (Default|CheckNexttoBulbState _sockettile))))