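; Cable actor that plays an electricity effect travelling between the join meshes of its Start and End objects.
; On BeginPlay it caches both mesh world locations, then a timeline lerps the Niagara component between them.
; When the timeline finishes it calls OnEndReached and destroys itself after a short delay.
; An alternative SplineMove event moves the effect along a two-point spline but is not called in this graph.
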(event Custom|StartElectricityFX
  (Variables|FX|SetLocations (Utilities|Array|MakeArray (Transformation|GetWorldLocation (Variables|/Game/Grid/BP_SocketTile.BP_SocketTile_C|GetCableJoinMesh (Variables|Default|GetStart))) (Transformation|GetWorldLocation (Variables|/Game/Grid/BP_SocketTile.BP_SocketTile_C|GetCableJoinMesh (Variables|Default|GetEnd)))))
  (CallFunction|MoveBetween))

(event Custom|MoveBetween
  (bind _locations (Variables|FX|GetLocations))
  (bind _movementalpha (Timeline|MoveToPosition PlayFromStart)
    (:Update
      (Transformation|SetWorldLocation (Variables|Default|GetNiagara) (Math|Vector|Lerp(Vector) (Utilities|Array|Get(acopy) _locations) (Utilities|Array|Get(acopy) _locations 1) _movementalpha) false false))
    (:Finished
      (Default|CallOnEndReached)
      (Utilities|FlowControl|Delay 0.5)
      (Actor|DestroyActor))))

(event Custom|SplineMove
  (bind _spline (Variables|Default|GetSpline))
  (bind _locations (Variables|FX|GetLocations))
  (Spline|SetLocationatSplinePoint _spline 0 (Utilities|Array|Get(acopy) _locations) "Local" true)
  (Spline|SetLocationatSplinePoint _spline 1 (Utilities|Array|Get(acopy) _locations 1) "Local" true)
  (bind _movementalpha (Timeline|Timeline_0 PlayFromStart)
    (:Update
      (Transformation|SetRelativeLocation (Variables|Default|GetNiagara) (Spline|GetLocationatDistanceAlongSpline (Variables|Default|GetSpline) (Math|Float|Lerp 0.0 (Spline|GetSplineLength (Variables|Default|GetSpline)) _movementalpha) "Local") false false))))

(event EventBeginPlay
  (|CallParentFunction)
  (CallFunction|StartElectricityFX))

(fn ConstructionScript)