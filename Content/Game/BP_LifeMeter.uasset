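; BP_LifeMeter is an in-world life display that tracks the player's remaining lives.
; On Init it caches the game mode and spawns a vertical column of BP_Life actors downward from its root, one per initial life from the game settings.
; LoseLife decrements the counter, hides the first still-visible life mesh from the top, and fires the OnLose dispatcher when none remain.
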(event Custom|Init
  (bind _asbp_game_mode (Utilities|Casting|CastToBP_GameMode (Game|GetGameMode)))
  (Variables|Default|SetGM _asbp_game_mode)
  (CallFunction|SpawnLives))

(fn ConstructionScript)

(fn SpawnLives
  (bind _out_row (CallFunction|GetGameSettings))
  (bind _defaultsceneroot (Variables|Default|GetDefaultSceneRoot))
  (bind _initiallives (Utilities|Struct|BreakS_GameSettings _out_row))
  (bind _returnvalue (Transformation|GetWorldLocation _defaultsceneroot))
  (bind (_x _y _z) (Math|Vector|BreakVector _returnvalue))
  (for _index (range 0 (- _initiallives 1))
    (bind _returnvalue_2 (Game|SpawnActorfromClass "/Game/Game/BP_Life.BP_Life_C" (Math|Transform|MakeTransform (Math|Vector|MakeVector _x _y (- _z (* (Math|Conversions|ToFloat(Integer) _index) (Variables|Default|GetDistanceBetweenLives))))) "Undefined" 0 0))
    (Utilities|Array|Add (Variables|Lives|GetLives) _returnvalue_2))
  (bind _output_get (Variables|Lives|SetLifeCounter _initiallives))
  (Development|PrintString (Utilities|String|Append "Live: " (Utilities|String|ToString(Integer) _output_get))))

(fn LoseLife
  (bind _result (Math|Integer|DecrementInt (Variables|Lives|GetLifeCounter))
    (:%20%20
      (bind _array_element (Utilities|Array|ForEachLoopwithBreak (Variables|Lives|GetLives) :!label _label)
        (:LoopBody
          (if (Variables|/Script/Engine.SceneComponent|GetbVisible (Variables|/Game/Game/BP_Life.BP_Life_C|GetStaticMesh _array_element))
            (Rendering|SetVisibility (Variables|/Game/Game/BP_Life.BP_Life_C|GetStaticMesh _array_element) false false)
            (goto _label Break)))
        (:Completed
          (if (<= _result 0)
            (Default|CallOnLose)
            (else
              (Development|PrintString (Utilities|String|Append "Lives Left: " (Utilities|String|ToString(Integer) _result))))))))))