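; BP_Fire is a fire VFX actor that plays when the player character reports a reached streak.
; BeginPlay binds PlayFireVFX to the character's streak event and hides both static meshes.
; PlayFireVFX ignores the streak level, shows the meshes, and plays a timeline that offsets the root's height and yaw from the transform captured at trigger time.
; The meshes hide again when the timeline finishes.
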(event Custom|PlayFireVFX
  (params (StreakLevel :type Integer))
  (bind _defaultsceneroot (Variables|Default|GetDefaultSceneRoot))
  (bind _defaultsceneroot_2 (Variables|Default|GetDefaultSceneRoot))
  (Variables|Animations|SetInitLocation (Transformation|GetWorldLocation _defaultsceneroot))
  (Variables|Animations|SetInitRotation (Transformation|GetWorldRotation _defaultsceneroot))
  (Rendering|SetVisibility (Variables|Default|GetStaticMesh) true true)
  (Rendering|SetVisibility (Variables|Default|GetStaticMesh1) true true)
  (bind _alpha (Timeline|Timeline_0 PlayFromStart)
    (:Update
      (Transformation|SetWorldLocation _defaultsceneroot_2 (Math|Vector|MakeVector (.X (Math|Vector|BreakVector (Variables|Animations|GetInitLocation))) (.Y (Math|Vector|BreakVector (Variables|Animations|GetInitLocation))) (+ (.Z (Math|Vector|BreakVector (Variables|Animations|GetInitLocation))) (* _alpha (Variables|Animations|GetLocationMultiplier)))) false false)
      (Transformation|SetWorldRotation _defaultsceneroot_2 (Math|Rotator|MakeRotator (.Roll (Math|Rotator|BreakRotator (Variables|Animations|GetInitRotation))) (.Pitch (Math|Rotator|BreakRotator (Variables|Animations|GetInitRotation))) (+ (.Yaw (Math|Rotator|BreakRotator (Variables|Animations|GetInitRotation))) (* _alpha (Variables|Animations|GetRotationMultiplier)))) false false))
    (:Finished
      (Rendering|SetVisibility (Variables|Default|GetStaticMesh) false true)
      (Rendering|SetVisibility (Variables|Default|GetStaticMesh1) false true))))

(event EventBeginPlay
  (EventDispatchers|BindEventtoOnStreakReached (CallFunction|GetPlayerCharacter) (delegate Custom|PlayFireVFX))
  (Rendering|SetVisibility (Variables|Default|GetStaticMesh) false true)
  (Rendering|SetVisibility (Variables|Default|GetStaticMesh1) false true))

(fn ConstructionScript)